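; BP_EnemySpawner is an actor that spawns BP_Enemy for the waves of the round-based top-down game mode.
; A looping timer checks GM_TopDown for round state, the alive cap and enemies remaining in the wave.
; When all pass, it spawns an enemy at a random entry of SpawnLocations and updates the game mode's counters.
; Otherwise, it asks the game mode to check whether the round has ended.
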(event Custom|TrySpawnEnemy
  (bind _spawnlocations (Variables|Default|GetSpawnLocations))
  (bind _asgm_top_down (Utilities|Casting|CastToGM_TopDown (Game|GetGameMode)))
  (if (and (and (< (Variables|/Game/Blueprints/Core/GM_TopDown.GM_TopDown_C|GetEnemiesAlive _asgm_top_down) (Variables|Default|GetMaxAliveEnemies)) (Utilities|Enum|Equal(Enum) (Variables|/Game/Blueprints/Core/GM_TopDown.GM_TopDown_C|GetCurrentGameState _asgm_top_down) "NewEnumerator0")) (> (Variables|/Game/Blueprints/Core/GM_TopDown.GM_TopDown_C|GetEnemiesRemainingTotal _asgm_top_down) 0))
    (Game|SpawnActorfromClass "/Game/Blueprints/Actors/BP_Enemy.BP_Enemy_C" (Math|Transform|MakeTransform (Utilities|Array|Get(acopy) _spawnlocations (Math|Random|RandomIntegerinRange 0 (Utilities|Array|LastIndex _spawnlocations)))) "Undefined" "MultiplyWithRoot" 0 0)
    ;[0.15 0.15 0.15 0.5] Actualizamos las variables del GameManager
    (bind _asgm_top_down_2 (Utilities|Casting|CastToGM_TopDown (Game|GetGameMode)))
    (Variables|/Game/Blueprints/Core/GM_TopDown.GM_TopDown_C|SetEnemiesRemainingTotal _asgm_top_down_2 (- (Variables|/Game/Blueprints/Core/GM_TopDown.GM_TopDown_C|GetEnemiesRemainingTotal _asgm_top_down_2) 1))
    (Variables|/Game/Blueprints/Core/GM_TopDown.GM_TopDown_C|SetEnemiesAlive _asgm_top_down_2 (+ (Variables|/Game/Blueprints/Core/GM_TopDown.GM_TopDown_C|GetEnemiesAlive _asgm_top_down_2) 1))
    (else
      (bind _asgm_top_down_3 (Utilities|Casting|CastToGM_TopDown (Game|GetGameMode)))
      (Default|CheckRoundEnd _asgm_top_down_3))))

(event EventBeginPlay
  (Utilities|Time|SetTimerbyEvent (delegate Custom|TrySpawnEnemy) (Variables|Default|GetSpawnInterval) true))

(event Collision|EventActorBeginOverlap
  (params (OtherActor :type Actor%20Object%20Reference)))

(event EventTick
  (params (DeltaSeconds :type Float%20%28single-precision%29)))

(fn ConstructionScript)