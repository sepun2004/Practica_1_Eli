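; BP_Enemy is a top-down enemy that chases the player and reports its death to the game mode.
; Tick reissues AIMoveTo toward the player every frame, followed by a close-range distance check that leads to no action, with damage-related nodes left unconnected.
; BeginPlay binds the health component's OnDeath to a handler that decrements GM_TopDown's EnemiesAlive count and destroys the actor.
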(event Custom|OnDeath_Event
  (bind _asgm_top_down (Utilities|Casting|CastToGM_TopDown (Game|GetGameMode)))
  (Variables|/Game/Blueprints/Core/GM_TopDown.GM_TopDown_C|SetEnemiesAlive _asgm_top_down (- (Variables|/Game/Blueprints/Core/GM_TopDown.GM_TopDown_C|GetEnemiesAlive _asgm_top_down) 1))
  (Actor|DestroyActor))

(event EventBeginPlay
  (EventDispatchers|AssignOnDeath (Variables|Default|GetBPC_HealthComponent) (delegate Custom|OnDeath_Event)))

(event Collision|EventActorBeginOverlap
  (params (OtherActor :type Actor%20Object%20Reference)))

(event EventTick
  (params (DeltaSeconds :type Float%20%28single-precision%29))
  (bind _returnvalue (Game|GetPlayerCharacter 0))
  (bind _self self)
  (AI|AIMoveTo _self "0, 0, 0" _returnvalue 0.0 false
    (:then
      (if (< (Transformation|GetDistanceTo _returnvalue _self) 1.5e+02)
        _))))

(fn ConstructionScript)